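; Actor component for BP_PlayerCharacter that implements a toggleable slow-motion ability, "Codename".
; Activation applies camera post-process settings and lowers global time dilation and audio pitch, either instantly or stepped down by a looping timer.
; Unless IncludePlayer is set, the player's CustomTimeDilation is inverted to keep normal speed.
; Toggling off or DeactivateAbility restores defaults without clearing the lerp timer; spring-arm camera code is unconnected.
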(event `LerpStart`
  (bind _currentvalue (`self.CurrentValue`))
  ;[1 1 1] Lerp Slomotion
  (bind _output_get (set `self.CurrentValue` (- (`self.CurrentValue`) (`self.LerpSpeed`))))
  (if (<= _output_get (`self.SlowMotionValue`))
    (`KismetSystemLibrary.K2_ClearAndInvalidateTimerHandle` (stale `ActivateCodename` _returnvalue_3))
    (else
      (`GameplayStatics.SetGlobalTimeDilation` _currentvalue)
      (`GameplayStatics.SetGlobalPitchModulation` _currentvalue)
      (if (not (`self.IncludePlayer?`))
        (set `Actor.CustomTimeDilation` (/ 1.0 (`self.CurrentValue`)) (`self.PlayerRef`))))))

(event `ActivateCodename`
  (bind _returnvalue (`self.GetOwner`))
  (bind _slowmotionvalue (`self.SlowMotionValue`))
  (bind _returnvalue_2 (`Actor.GetComponentByClass` (`self.PlayerRef`) "/Script/Engine.CameraComponent"))
  (`/Engine/EditorBlueprintResources/StandardMacros.IsValid` _returnvalue
    (:`Is Valid`
      (bind _asbp_player_character (cast `/Game/AlexBrusow_GD_Project/Core/Character/BP_PlayerCharacter` _returnvalue))
      (set `self.PlayerRef` _asbp_player_character)
      (`|ExecutionSequence`
        (:`then_0`
          (if (not (`self.IsSlowTimeActive?`))
            (set `self.IsSlowTimeActive?` true)
            (`/Engine/EditorBlueprintResources/StandardMacros.IsValid` _returnvalue_2
              (:`Is Valid`
                (set `CameraComponent.PostProcessSettings` (`self.PPSettings`) _returnvalue_2)
                (if (`self.Lerp?`)
                  ;[1 1 1] Lerp Slomotion
                  (set `self.CurrentValue` 1.0)
                  (bind _returnvalue_3 (`KismetSystemLibrary.K2_SetTimerDelegate` (delegate `LerpStart`) (`self.LerpSpeed`) true))
                  (else
                    ;[1 1 1] Instant Slomotion
                    (`GameplayStatics.SetGlobalTimeDilation` _slowmotionvalue)
                    (`GameplayStatics.SetGlobalPitchModulation` _slowmotionvalue)
                    (if (not (`self.IncludePlayer?`))
                      (set `Actor.CustomTimeDilation` (/ 1.0 (`self.SlowMotionValue`)) (`self.PlayerRef`)))))))
            (else
              (set `self.IsSlowTimeActive?` false :!label _label)
              (`/Engine/EditorBlueprintResources/StandardMacros.IsValid` _returnvalue_2
                (:`Is Valid`
                  (set `CameraComponent.PostProcessSettings` (struct) _returnvalue_2))
                (:`Is Not Valid`
                  _))
              ;[1 1 1] Reset to defaults
              (`GameplayStatics.SetGlobalTimeDilation` 1.0)
              (`GameplayStatics.SetGlobalPitchModulation` 1.0)
              (set `Actor.CustomTimeDilation` 1.0 (`self.PlayerRef`)))))
        (:`then_1`
          (`/Engine/EditorBlueprintResources/StandardMacros.FlipFlop`))))))

(event `DeactivateAbility`
  (goto _label))