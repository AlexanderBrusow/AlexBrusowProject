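; Base weapon actor for the AIShooter weapon system, with mesh and anim class set from WeaponConfig.
; It starts Dropped with physics and an overlap sphere that toggles an info widget for the player.
; Interact passes config and actor to the component's PickUpWeaponMessage, while the Equipped state disables physics and collision and destroys the widget.
; WeaponMuzzleEffects spawns a beam trail to the given end point and briefly flashes the muzzle.
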(event `self.ReceiveBeginPlay`
  (bind ((`name_10_107A7A6D40D768433A7133BBDFB1B1B0` _name) (`CurrentAmmo_5_373CD79A4F8E51F2B87D28A459E5ABF4` _currentammo) (`Icon_18_5892FC294F2F5BC5D62987BA699E6285` _icon) (`WeaponModeFire_22_7D5DD0B44B585C16BDFD4AAC424A3710` _weaponmodefire)) (break `/Game/AIShooter/System/WeaponSystem/Blueprint/S_WeaponConfig` (`self.WeaponConfig`)))
  ;[0 1 0.856 1 30] Beginplay
  (`self.SetWeaponState` "NewEnumerator0")
  (bind _aswb_interact_weapon (cast `/Game/AIShooter/System/WeaponSystem/Widget/WB_InteractWeapon` (`WidgetComponent.GetUserWidgetObject` (`self.Widget`))))
  (bind _output_get (set `self.WidgetWeapon` _aswb_interact_weapon))
  (`/Game/AIShooter/System/WeaponSystem/Widget/WB_InteractWeapon.SetWidgetConfig` _output_get _icon (`KismetStringLibrary.Conv_StringToName` _name) _currentammo _weaponmodefire))

(event `self.Sphere.OnComponentBeginOverlap`
  (params (OverlappedComponent :type "PrimitiveComponent Object Reference") (OtherActor :type "Actor Object Reference") (OtherComp :type "PrimitiveComponent Object Reference") (OtherBodyIndex :type Integer) (bFromSweep :type Boolean) (SweepResult :type "HitResult Structure (by ref)"))
  (bind _widgetweapon (`self.WidgetWeapon`))
  ;[1 0 0.6093 1 30] Overlap
  (if (== OtherActor (`GameplayStatics.GetPlayerCharacter` 0))
    (`/Engine/EditorBlueprintResources/StandardMacros.IsValid` _widgetweapon
      (:`Is Valid`
        (`/Game/AIShooter/System/WeaponSystem/Widget/WB_InteractWeapon.VisibilityOn` _widgetweapon)))))

(event `/Game/AIShooter/System/WeaponSystem/Blueprint/BP_WeaponInterface.Interact`
  (params (Component :type "/Game/AIShooter/System/Component/BP_AIShooterComponent Object Reference") (PlayerCharacter :type "Character Object Reference"))
  ;[1 0 0.6093 1 30] Overlap
  (message `/Game/AIShooter/System/WeaponSystem/Blueprint/BP_WeaponInterface.PickUpWeapon` Component (`self.WeaponConfig`) PlayerCharacter self))

(event `RemoveWidget`
  (bind _widget (`self.Widget`))
  ;[0 0.339 1] Remove Widget
  (`/Engine/EditorBlueprintResources/StandardMacros.IsValid` _widget
    (:`Is Valid`
      (`ActorComponent.K2_DestroyComponent` _widget))))

(event `self.Sphere.OnComponentEndOverlap`
  (params (OverlappedComponent :type "PrimitiveComponent Object Reference") (OtherActor :type "Actor Object Reference") (OtherComp :type "PrimitiveComponent Object Reference") (OtherBodyIndex :type Integer))
  (bind _widgetweapon (`self.WidgetWeapon`))
  ;[1 0 0.6093 1 30] Overlap
  (if (== OtherActor (`GameplayStatics.GetPlayerCharacter` 0))
    (`/Engine/EditorBlueprintResources/StandardMacros.IsValid` _widgetweapon
      (:`Is Valid`
        (`/Game/AIShooter/System/WeaponSystem/Widget/WB_InteractWeapon.VisibilityOff` _widgetweapon)))))

(event `WeaponMuzzleEffects`
  (params (LocationEnd :type "Vector Structure"))
  (bind _muzzle (`self.Muzzle`))
  ;[1 0.0648 0] Active Muzzle Effect Fire
  (bind _returnvalue (`GameplayStatics.SpawnEmitterAtLocation` "/Game/AIShooter/Demo/Weapon/Effects/P_AssaultRifle_Trail.P_AssaultRifle_Trail" (`SceneComponent.K2_GetComponentLocation` _muzzle) (`SceneComponent.K2_GetComponentRotation` _muzzle) (5.0 5.0 5.0)))
  (`FXSystemComponent.SetVectorParameter` _returnvalue "ShockBeamEnd" LocationEnd)
  (`SceneComponent.SetVisibility` (`self.P_AssaultRifle_MF`) true false)
  (`KismetSystemLibrary.Delay` 0.2)
  (`SceneComponent.SetVisibility` (`self.P_AssaultRifle_MF`) false false))

(fn `SetWeaponState`
  (params (WeaponState :type "/Game/AIShooter/System/WeaponSystem/Blueprint/E_WeaponState Enum" :default "NewEnumerator0"))
  (bind _skeletalmesh (`self.SkeletalMesh`))
  (bind _skeletalmesh_2 (`self.SkeletalMesh`))
  (switch `/Game/AIShooter/System/WeaponSystem/Blueprint/E_WeaponState` WeaponState
    (:`NewEnumerator0`
      (`PrimitiveComponent.SetCollisionProfileName` (`self.Sphere`) "OverlapAllDynamic" true)
      (`PrimitiveComponent.SetSimulatePhysics` _skeletalmesh true)
      (`PrimitiveComponent.SetCollisionProfileName` _skeletalmesh "WeaponDrop" true))
    (:`NewEnumerator1`
      (`PrimitiveComponent.SetCollisionProfileName` (`self.Sphere`) "NoCollision" true)
      (`PrimitiveComponent.SetSimulatePhysics` _skeletalmesh_2 false)
      (`PrimitiveComponent.SetCollisionProfileName` _skeletalmesh_2 "NoCollision" true)
      (`SceneComponent.ResetRelativeTransform` (`self.SkeletalMesh`))
      (`self.RemoveWidget`))))

(fn `UserConstructionScript`
  (bind _skeletalmesh (`self.SkeletalMesh`))
  (bind (_name _skeletalmesh_2 _animationblueprint) (break `/Game/AIShooter/System/WeaponSystem/Blueprint/S_WeaponConfig` (`self.WeaponConfig`)))
  (`SkinnedMeshComponent.SetSkinnedAssetAndUpdate` _skeletalmesh _skeletalmesh_2 true)
  (`SkeletalMeshComponent.SetAnimInstanceClass` _skeletalmesh _animationblueprint))