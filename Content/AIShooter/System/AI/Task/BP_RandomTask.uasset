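; Behavior Tree service, despite its Task name, that randomizes the Number blackboard key each time it activates.
; It normally rolls 0 to 2, but a value of 2 is held for three further activations, counted by NumberAmount.
; On the following activation it resets the counter and rolls only 0 or 1, so 2 cannot immediately recur.
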(event `self.ReceiveActivationAI`
  (params (OwnerController :type "AIController Object Reference") (ControlledPawn :type "Pawn Object Reference"))
  (if (== (`BTFunctionLibrary.GetBlackboardValueAsInt` (`self.Number`)) 2)
    (if (== (`self.NumberAmount`) 3)
      (set `self.NumberAmount` 0)
      (`BTFunctionLibrary.SetBlackboardValueAsInt` (`self.Number`) (`KismetMathLibrary.RandomIntegerInRange` 0 1))
      (else
        (`/Engine/EditorBlueprintResources/StandardMacros.IncrementInt` (`self.NumberAmount`)
          (:`  `
            (`BTFunctionLibrary.SetBlackboardValueAsInt` (`self.Number`) 2)))))
    (else
      (`BTFunctionLibrary.SetBlackboardValueAsInt` (`self.Number`) (`KismetMathLibrary.RandomIntegerInRange` 0 2)))))