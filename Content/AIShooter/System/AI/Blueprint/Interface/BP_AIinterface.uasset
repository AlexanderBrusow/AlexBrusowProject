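; Blueprint interface declaring the calls an AI shooter character exposes, with no logic of its own.
; Queries cover target, team ID, enemy checks, next movement location and initial move.
; Commands drive weapon equipping, firing, melee, stance, velocity and health bar visibility.
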(fn `EquipWeapon`
  (params (Equip :type Boolean)))

(fn `Fire`
  (params (`Enable?` :type Boolean)))

(fn `GetTarget`
  (returns (Target :type "/Game/AIShooter/System/AI/Blueprint/Enumeration/E_Target Enum"))
  (return "NewEnumerator0"))

(fn `GetTeamID`
  (returns (TeamID :type "/Game/AIShooter/System/AI/Blueprint/Enumeration/E_TeamName Enum"))
  (return "NewEnumerator0"))

(fn `InitialMove`
  (returns (InitalMove :type "/Game/AIShooter/System/AI/Blueprint/Enumeration/E_InitialMove Enum"))
  (return "NewEnumerator2"))

(fn `IsEnemy?`
  (params (`Team Name` :type "/Game/AIShooter/System/AI/Blueprint/Enumeration/E_TeamName Enum" :default "NewEnumerator0"))
  (returns (`Enemy?` :type Boolean))
  (return false))

(fn `Melee`)

(fn `NextMovementLocation`
  (returns (Location :type "Vector Structure"))
  (return (0.0 0.0 0.0)))

(fn `SetStance`
  (params (Stance :type "/Game/AIShooter/System/AI/Blueprint/Enumeration/E_SetStance Enum" :default "NewEnumerator0"))
  (return))

(fn `SetVelocity`
  (params (Value :type "Float (double-precision)")))

(fn `VisibilityHealthBar`
  (params (`On/Off` :type Boolean)))