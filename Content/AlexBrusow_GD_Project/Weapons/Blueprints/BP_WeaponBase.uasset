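; Base weapon Blueprint that handles shooting, reloading and reserve ammo for the player, delegating firing and magazine count to an EBBarrel component.
; While firing, the barrel moves to where the camera ray crosses the muzzle plane and takes the camera rotation, so shots follow the aim.
; Each shot triggers muzzle flash and montages; StartReload blocks shooting, and EndReload transfers reserve ammo and unblocks it.
; Tick also draws optional aim debug and prints ammo while equipped.
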(event `StartShoot`
  ;[1 1 1] Start & Stop Shoot Event
  (if (not (`EBBarrel.ShootingBlocked` (`self.EBBarrel`)))
    (set `self.bIsShooting` true)
    (`self.Update Barrel Location`)
    (`EBBarrel.Shoot` (`self.EBBarrel`) true)))

(event `self.ReceiveBeginPlay`
  (set `self.CurrentRemainingAmmo` (`self.MaxRemainingAmmo`))
  (add `EBBarrel.ShotFired` (`self.EBBarrel`) (delegate `OnShotFired`)))

(event `OnShotFired`
  (`ActorComponent.Activate` (`self.MuzzleFlash`) true)
  (`|PlayMontage` (`self.WeaponSkeletalMesh`) (`self.WeaponShotMontage`)
    (:`then`
      (`|PlayMontage` (`Character.Mesh` (`self.PlayerRef`)) (`self.PlayerShootMontage`)))))

(event `StopShoot`
  ;[1 1 1] Start & Stop Shoot Event
  (set `self.bIsShooting` false)
  (`EBBarrel.Shoot` (`self.EBBarrel`) false)
  (`SceneComponent.K2_SetWorldTransform` (`self.EBBarrel`) (`SceneComponent.K2_GetComponentToWorld` (`self.MuzzleLocation`)) false false))

(event `self.ReceiveTick`
  (params (DeltaSeconds :type "Float (single-precision)"))
  (`|ExecutionSequence`
    (:`then_0`
      (`self.DebugDraw`)
      (if (`self.bIsShooting`)
        (`self.Update Barrel Location`)))
    (:`then_1`
      (if (`/Game/AlexBrusow_GD_Project/Core/Character/BP_PlayerCharacter.bIsWeaponEquipped` (`self.PlayerRef`))
        (`KismetSystemLibrary.PrintString` (`KismetStringLibrary.Concat_StrStr` (`KismetStringLibrary.BuildString_Int` "MagazineSize" " " (`self.MagazineSize`) " ") (`KismetStringLibrary.BuildString_Int` "Max Remaining Ammo" " " (`self.MaxRemainingAmmo`) " ") (`KismetStringLibrary.BuildString_Int` "Current Remaining Ammo" " " (`self.CurrentRemainingAmmo`) " ") (`KismetStringLibrary.BuildString_Int` "Cycle Ammo Count" " " (`EBBarrel.GetAmmoCount` (`self.EBBarrel`) true) " ")) true true (struct :`G` 0.66 :`B` 1.0 :`A` 1.0) 0.0)))))

(fn `DebugDraw`
  (bind _returnvalue (`SceneComponent.K2_GetComponentLocation` (`self.MuzzleLocation`)))
  (bind _returnvalue_2 (`SceneComponent.K2_GetComponentLocation` (`self.EBBarrel`)))
  (if (`self.bEnableDebug`)
    (`KismetSystemLibrary.DrawDebugLine` _returnvalue _returnvalue_2 (struct :`R` 0.838542 :`B` 0.716443 :`A` 1.0) 0.0 2.0)
    (`KismetSystemLibrary.DrawDebugSphere` _returnvalue 20.0 12 (struct :`R` 1.0 :`G` 0.485008 :`A` 1.0) 0.0 1.0)
    (`KismetSystemLibrary.DrawDebugSphere` _returnvalue_2 10.0 12 (struct :`R` 0.023903 :`B` 1.0 :`A` 1.0) 0.0 1.0)))

(fn `EndReload`
  (bind _ebbarrel (`self.EBBarrel`))
  (bind _ebbarrel_2 (`self.EBBarrel`))
  (if (< (`self.RequiredAmmoCount`) (`self.CurrentRemainingAmmo`))
    (set `self.CurrentRemainingAmmo` (- (`self.CurrentRemainingAmmo`) (`self.RequiredAmmoCount`)))
    (`EBBarrel.SetAmmo` (`self.EBBarrel`) (+ (`EBBarrel.GetAmmoCount` _ebbarrel_2 true) (`self.RequiredAmmoCount`)) true false false (`EBBarrel.GetAmmo` _ebbarrel_2 true))
    (else
      (`EBBarrel.SetAmmo` _ebbarrel (+ (`EBBarrel.GetAmmoCount` (`self.EBBarrel`) true) (`self.CurrentRemainingAmmo`)) true false false (`EBBarrel.GetAmmo` _ebbarrel true))
      (set `self.CurrentRemainingAmmo` 0)))
  (set `EBBarrel.ShootingBlocked` false (`self.EBBarrel`))
  (set `self.bIsReloading` false)
  (`KismetSystemLibrary.PrintString` "Reloading"))

(fn `GetCurrentMagazineAmmo`
  (returns (CurrentMagazineAmmo :type Integer))
  (return (`EBBarrel.GetAmmoCount` (`self.EBBarrel`) true)))

(fn `GetCurrentRemainingAmmo`
  (returns (CurrentRemainingAmmo :type Integer))
  (return (`self.CurrentRemainingAmmo`)))

(fn `GetRequiredAmmo`
  (bind _magazinesize (`self.MagazineSize`))
  (set `self.RequiredAmmoCount` (`KismetMathLibrary.Clamp` (- _magazinesize (`EBBarrel.GetAmmoCount` (`self.EBBarrel`) true)) 0 _magazinesize))
  (return))

(fn `StartReload`
  (if (`self.bIsReloading`)
    (`KismetSystemLibrary.PrintString` "Reloading")
    (elif (> (`self.CurrentRemainingAmmo`) 0)
      (`self.GetRequiredAmmo`)
      (if (== (`self.RequiredAmmoCount`) 0)
        (`KismetSystemLibrary.PrintString` "Ammo Full")
        (else
          (set `EBBarrel.ShootingBlocked` true (`self.EBBarrel`))
          (set `self.bIsReloading` true)
          (`Character.PlayAnimMontage` (`self.PlayerRef`) (`self.PlayerReloadMontage`) (`self.ReloadSpeed`) "None")
          (`AudioComponent.Play` (`self.ReloadSound`) 0.0)))
      (else
        (`KismetSystemLibrary.PrintString` "NO AMMO")))))

(fn `Update Barrel Location`
  (bind _muzzlelocation (`self.MuzzleLocation`))
  (bind _followcamera (`/Game/AlexBrusow_GD_Project/Core/Character/BP_PlayerCharacter.FollowCamera` (`self.PlayerRef`)))
  (bind _returnvalue (`SceneComponent.K2_GetComponentLocation` _followcamera))
  (`SceneComponent.K2_SetWorldLocation` (`self.EBBarrel`) (`.Intersection` (`KismetMathLibrary.LinePlaneIntersection_OriginNormal` _returnvalue (+ _returnvalue (* (`SceneComponent.GetForwardVector` _followcamera) 1000.0)) (`SceneComponent.K2_GetComponentLocation` _muzzlelocation) (`SceneComponent.GetForwardVector` _muzzlelocation))) false false)
  (`SceneComponent.K2_SetWorldRotation` (`self.EBBarrel`) (`SceneComponent.K2_GetComponentRotation` (`/Game/AlexBrusow_GD_Project/Core/Character/BP_PlayerCharacter.FollowCamera` (`self.PlayerRef`))) false false))

(fn `UserConstructionScript`)