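; Base weapon for the player character that aligns the ballistic barrel (EBBarrel) with the follow camera's aim.
; UpdateBarrelLocation extends the parent, caches the owning player, then moves the barrel to where the camera ray crosses the muzzle plane, matching camera rotation.
; While shooting, Tick maps crosshair spread size to normalized barrel spread and prints debug ammo counts if a weapon is equipped.
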(event `self.Update Barrel Location`
  (bind _muzzlelocation (`self.MuzzleLocation`))
  (bind _followcamera (`/Game/AlexBrusow_GD_Project/Core/Character/BP_PlayerCharacter.FollowCamera` (`self.PlayerWeaponOwner`)))
  (bind _returnvalue (`SceneComponent.K2_GetComponentLocation` _followcamera))
  (`parent.Update Barrel Location`)
  (bind _asbp_player_character (cast `/Game/AlexBrusow_GD_Project/Core/Character/BP_PlayerCharacter` (`self.WeaponOwner`)))
  (set `self.PlayerWeaponOwner` _asbp_player_character)
  (`SceneComponent.K2_SetWorldLocation` (`self.EBBarrel`) (`.Intersection` (`KismetMathLibrary.LinePlaneIntersection_OriginNormal` _returnvalue (+ _returnvalue (* (`SceneComponent.GetForwardVector` _followcamera) 1000.0)) (`SceneComponent.K2_GetComponentLocation` _muzzlelocation) (`SceneComponent.GetForwardVector` _muzzlelocation))) false false)
  (`SceneComponent.K2_SetWorldRotation` (`self.EBBarrel`) (`SceneComponent.K2_GetComponentRotation` (`/Game/AlexBrusow_GD_Project/Core/Character/BP_PlayerCharacter.FollowCamera` (`self.PlayerWeaponOwner`))) false false))

(event `self.ReceiveTick`
  (params (DeltaSeconds :type "Float (single-precision)"))
  (bind _playerweaponowner (`self.PlayerWeaponOwner`))
  (if (`self.bIsShooting`)
    (`|ExecutionSequence`
      (:`then_0`
        ;[1 1 1] Set Spread from CrosshairRange
        (set `EBBarrel.Spread` (`KismetMathLibrary.NormalizeToRange` (`/Game/AlexBrusow_GD_Project/Widgets/Crosshair/WBP_RiffleCrosshair.SpreadSize` (`/Game/AlexBrusow_GD_Project/Core/Character/BP_PlayerCharacter.CrosshairWidget` _playerweaponowner)) 0.0 50.0) (`self.EBBarrel`)))
      (:`then_1`
        ;[1 1 1] Debug strings
        (if (`/Game/AlexBrusow_GD_Project/Core/Character/BP_PlayerCharacter.bIsWeaponEquipped` _playerweaponowner)
          (`KismetSystemLibrary.PrintString` (`KismetStringLibrary.Concat_StrStr` (`KismetStringLibrary.BuildString_Int` "MagazineSize" " " (`self.MagazineSize`) " ") (`KismetStringLibrary.BuildString_Int` "Max Remaining Ammo" " " (`self.MaxRemainingAmmo`) " ") (`KismetStringLibrary.BuildString_Int` "Current Remaining Ammo" " " (`self.CurrentRemainingAmmo`) " ") (`KismetStringLibrary.BuildString_Int` "Cycle Ammo Count" " " (`EBBarrel.GetAmmoCount` (`self.EBBarrel`) true) " ")) true true (struct :`G` 0.66 :`B` 1.0 :`A` 1.0) 0.0))))))

(fn `UserConstructionScript`
  (`parent.UserConstructionScript`))