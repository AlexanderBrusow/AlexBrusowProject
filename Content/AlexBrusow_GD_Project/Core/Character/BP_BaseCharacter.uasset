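; Base character Blueprint that provides health, damage handling and death for the characters derived from it.
; AnyDamage subtracts from clamped current health while it is above zero, then prints a debug message and triggers OnDeath when it runs out.
; OnDeath flags the character dead, calls OnDead, starts the death montage on a valid mesh and calls OnPostDead immediately, without waiting for completion.
; GetHealth returns health as a normalized fraction.
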(event `self.ReceiveAnyDamage`
  (params (Damage :type "Float (single-precision)") (DamageType :type "DamageType Object Reference") (InstigatedBy :type "Controller Object Reference") (DamageCauser :type "Actor Object Reference"))
  (bind _currenthealth (`self.CurrentHealth`))
  ;[1 1 1] Event Damage
  (if (> _currenthealth 0.0)
    (bind _output_get (set `self.CurrentHealth` (`KismetMathLibrary.FClamp` (- _currenthealth Damage) 0.0 (`self.MaxHealth`))))
    (if (<= _output_get 0.0)
      (`KismetSystemLibrary.PrintString` "DEAD!" true true (struct :`R` 1.0 :`B` 0.030305 :`A` 1.0) 3.0)
      (`self.OnDeath`))))

(event `OnDeath`
  (bind _mesh (`self.Mesh`))
  ;[1 1 1] Event OnDeath
  (set `self.bIsDead` true)
  (`self.OnDead`)
  (`/Engine/EditorBlueprintResources/StandardMacros.IsValid` _mesh
    (:`Is Valid`
      (`|PlayMontage` _mesh (`self.DeathMontage`)
        (:`then`
          (`self.OnPostDead`))))))

(fn `GetHealth`
  (returns (HealthRatio :type "Float (double-precision)"))
  (return (`KismetMathLibrary.FClamp` (/ (`self.CurrentHealth`) (`self.MaxHealth`)))))

(fn `UserConstructionScript`)