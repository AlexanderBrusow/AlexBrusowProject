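; Base weapon Blueprint for AI enemies that aims its barrel at the wielder's current target.
; It overrides UpdateBarrelLocation, calling the parent, then rotating EBBarrel to face the TargetEnemy held by the owning AI_BaseEnemy's controller.
; It also draws a debug arrow from the barrel, whose end is the scaled forward vector without the barrel location added.
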(event `self.Update Barrel Location`
  (bind _ebbarrel (`self.EBBarrel`))
  (`parent.Update Barrel Location`)
  (`KismetSystemLibrary.DrawDebugArrow` (`SceneComponent.K2_GetComponentLocation` _ebbarrel) (* (`SceneComponent.GetForwardVector` _ebbarrel) 100.0) 0.0 (struct :`R` 1.0 :`B` 0.198586 :`A` 1.0) 2.0 1.0)
  (bind _asai_base_enemy (cast `/Game/AlexBrusow_GD_Project/AI/BaseEnemy/AI_BaseEnemy` (`self.WeaponOwner`)))
  (bind _targetenemy (`/Game/AlexBrusow_GD_Project/AI/BaseEnemy/AIC_BaseEnemy.TargetEnemy` (`/Game/AlexBrusow_GD_Project/AI/BaseEnemy/AI_BaseEnemy.ControllerRef` _asai_base_enemy)))
  (`/Engine/EditorBlueprintResources/StandardMacros.IsValid` _targetenemy
    (:`Is Valid`
      (`SceneComponent.K2_SetWorldRotation` (`self.EBBarrel`) (`KismetMathLibrary.FindLookAtRotation` (`SceneComponent.K2_GetComponentLocation` (`self.EBBarrel`)) (`self.K2_GetActorLocation` _targetenemy)) false false))))

(fn `UserConstructionScript`
  (`parent.UserConstructionScript`))