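; BP_BasicGameMode is a game mode that declares a win once every enemy in its EnemiesToKill list has died.
; On BeginPlay it binds to the OnPostDead dispatcher of each valid enemy reference in that list.
; Each death increments KillCount, and OnWin is called when the count equals the full list length, including any entries skipped as invalid.
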(event `self.ReceiveBeginPlay`
  (for _array_element (`self.EnemiesToKill`)
    (bind _output (`|ConvertAsset` _array_element))
    (`/Engine/EditorBlueprintResources/StandardMacros.IsValid` _output
      (:`Is Valid`
        (add `/Game/AlexBrusow_GD_Project/Core/Character/BP_BaseCharacter.OnPostDead` _output (delegate `On PostDead Event`))))))

(event `On PostDead Event`
  (bind _result (`/Engine/EditorBlueprintResources/StandardMacros.IncrementInt` (`self.KillCount`))
    (:`  `
      (set `self.KillCount` _result)
      (if (== (`KismetArrayLibrary.Array_Length` (`self.EnemiesToKill`)) (`self.KillCount`))
        (`self.OnWin`)))))

(fn `UserConstructionScript`)