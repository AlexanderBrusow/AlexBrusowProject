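; Ceiling light actor that switches on while the player character is inside its trigger box.
; Box collision overlap events, filtered to BP_PlayerCharacter, set the point light to a fixed intensity on entry and to zero on exit.
; The construction script applies the Brightness, Color and SourceRadius variables to the light, so the initial intensity follows Brightness until an overlap overrides it.
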(event `self.BoxCollisionLamp.OnComponentBeginOverlap`
  (params (OverlappedComponent :type "PrimitiveComponent Object Reference") (OtherActor :type "Actor Object Reference") (OtherComp :type "PrimitiveComponent Object Reference") (OtherBodyIndex :type Integer) (bFromSweep :type Boolean) (SweepResult :type "HitResult Structure (by ref)"))
  (cast `/Game/AlexBrusow_GD_Project/Core/Character/BP_PlayerCharacter` OtherActor)
  (`LightComponent.SetIntensity` (`self.PointLight`) 1700.0))

(event `self.BoxCollisionLamp.OnComponentEndOverlap`
  (params (OverlappedComponent :type "PrimitiveComponent Object Reference") (OtherActor :type "Actor Object Reference") (OtherComp :type "PrimitiveComponent Object Reference") (OtherBodyIndex :type Integer))
  (cast `/Game/AlexBrusow_GD_Project/Core/Character/BP_PlayerCharacter` OtherActor)
  (`LightComponent.SetIntensity` (`self.PointLight`) 0.0))

(fn `UserConstructionScript`
  (bind _pointlight (`self.PointLight`))
  (`LightComponent.SetIntensity` _pointlight (`self.Brightness`))
  (`LightComponent.SetLightColor` _pointlight (`self.Color`) true)
  (`PointLightComponent.SetSourceRadius` _pointlight (`self.Source Radius`)))